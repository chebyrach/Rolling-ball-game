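; Pressure-button Blueprint that moves a linked Door vertically while a PhysicsBallBP overlaps its trigger Sphere.
; BeginPlay caches the Button and Door world locations as rest positions.
; Overlap begin plays a sound and runs ButtonTimeline forward; overlap end reverses it.
; Each timeline update feeds two elevation tracks into UpdateButton, which offsets both components in Z from their cached starts.
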(event OnComponentBeginOverlap(Sphere)
  (params (OverlappedComponent :type Primitive%20Component%20Object%20Reference) (OtherActor :type Actor%20Object%20Reference) (OtherComp :type Primitive%20Component%20Object%20Reference) (OtherBodyIndex :type Integer) (bFromSweep :type Boolean) (SweepResult :type Hit%20Result%20Structure%20%28by%20ref%29))
  (Utilities|Casting|CastToPhysicsBallBP OtherActor)
  (Audio|PlaySound2D "/Game/SmallSoundKit/SSKCue/FootstepsCue/S_Concrete_Mono_1_Cue.S_Concrete_Mono_1_Cue" 1.0 1.0 0.0 0 0)
  (bind (_direction _buttonelevation _doortimeline) (Timeline|ButtonTimeline Play)
    (:Update
      (CallFunction|UpdateButton _buttonelevation _doortimeline))))

(event OnComponentEndOverlap(Sphere)
  (params (OverlappedComponent :type Primitive%20Component%20Object%20Reference) (OtherActor :type Actor%20Object%20Reference) (OtherComp :type Primitive%20Component%20Object%20Reference) (OtherBodyIndex :type Integer))
  (Utilities|Casting|CastToPhysicsBallBP OtherActor)
  (bind (_direction _buttonelevation _doortimeline) (Timeline|ButtonTimeline Reverse)
    (:Update
      (CallFunction|UpdateButton _buttonelevation _doortimeline))))

(event EventBeginPlay
  (Variables|Default|SetStartDoorLocation (Transformation|GetWorldLocation (Variables|Default|GetDoor)))
  (Variables|Default|SetStartButtonLocation (Transformation|GetWorldLocation (Variables|Default|GetButton))))

(event EventTick
  (params (DeltaSeconds :type Float%20%28single-precision%29)))

(fn ConstructionScript)

(fn UpdateButton
  (params (ButtonElevation :type Float%20%28single-precision%29) (DoorElevation :type Float%20%28single-precision%29))
  (bind _startbuttonlocation (Variables|Default|GetStartButtonLocation))
  (bind _startdoorlocation (Variables|Default|GetStartDoorLocation))
  (bind (_x _y _z) (Math|Vector|BreakVector _startbuttonlocation))
  (bind (_x_2 _y_2 _z_2) (Math|Vector|BreakVector _startdoorlocation))
  (Utilities|FlowControl|Sequence
    (:then_0
      (Transformation|SetWorldLocation (Variables|Default|GetButton) (Math|Vector|MakeVector _x _y (+ _z ButtonElevation)) false false))
    (:then_1
      (Transformation|SetWorldLocation (Variables|Default|GetDoor) (Math|Vector|MakeVector _x_2 _y_2 (+ _z_2 DoorElevation)) false false))))