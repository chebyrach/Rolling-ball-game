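; Booster actor with a button that reacts to a PhysicsBallBP entering or leaving its sphere trigger; no boost force is applied here.
; On overlap it plays a concrete sound and plays ButtonTimeline, which it reverses when the ball leaves.
; Timeline updates call UpdateButton, which sets the button a fixed offset above its BeginPlay location, with no timeline value feeding the height.
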(event OnComponentBeginOverlap(Sphere)
  (params (OverlappedComponent :type Primitive%20Component%20Object%20Reference) (OtherActor :type Actor%20Object%20Reference) (OtherComp :type Primitive%20Component%20Object%20Reference) (OtherBodyIndex :type Integer) (bFromSweep :type Boolean) (SweepResult :type Hit%20Result%20Structure%20%28by%20ref%29))
  (Utilities|Casting|CastToPhysicsBallBP OtherActor)
  (Audio|PlaySound2D "/Game/SmallSoundKit/SSKCue/FootstepsCue/S_Concrete_Mono_1_Cue.S_Concrete_Mono_1_Cue" 1.0 1.0 0.0 0 0)
  (Timeline|ButtonTimeline Play
    (:Update
      (CallFunction|UpdateButton))))

(event OnComponentEndOverlap(Sphere)
  (params (OverlappedComponent :type Primitive%20Component%20Object%20Reference) (OtherActor :type Actor%20Object%20Reference) (OtherComp :type Primitive%20Component%20Object%20Reference) (OtherBodyIndex :type Integer))
  (Utilities|Casting|CastToPhysicsBallBP OtherActor)
  (Timeline|ButtonTimeline Reverse
    (:Update
      (CallFunction|UpdateButton))))

(event EventBeginPlay
  (Variables|Default|SetStartButtonLocation (Transformation|GetWorldLocation (Variables|Default|GetButton))))

(event Collision|EventActorBeginOverlap
  (params (OtherActor :type Actor%20Object%20Reference)))

(event EventTick
  (params (DeltaSeconds :type Float%20%28single-precision%29)))

(fn ConstructionScript)

(fn UpdateButton
  (bind _startbuttonlocation (Variables|Default|GetStartButtonLocation))
  (bind (_x _y _z) (Math|Vector|BreakVector _startbuttonlocation))
  (Transformation|SetWorldLocation (Variables|Default|GetButton) (Math|Vector|MakeVector _x _y (+ _z 1.0)) false false))