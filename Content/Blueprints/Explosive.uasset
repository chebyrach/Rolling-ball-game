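; Explosive pickup, a child of a pickup Blueprint, that blasts the player's physics ball away on pickup and is worth no points.
; BeginPlay turns off the number widget, sets explosion sound and particle on inherited variables, and plays a sparks sound at its location.
; OnPickup applies a constant-falloff, velocity-change radial impulse to the PhysicsBallBP's Ball from just below the actor, then calls the parent pickup logic.
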(event EventBeginPlay
  (Variables|Default|SetuseNumberWidget false)
  (Variables|Default|SetPoints 0)
  (Variables|Default|SetPickupSound "/Game/StarterContent/Audio/Explosion01.Explosion01")
  (Variables|Default|SetPickup%20particle "/Game/StarterContent/Particles/P_Explosion.P_Explosion")
  (Audio|PlaySoundatLocation "/Game/StarterContent/Audio/Fire_Sparks01_Cue.Fire_Sparks01_Cue" (Transformation|GetActorLocation) "0, 0, 0" 1.0 1.0 0.0 0 0 0)
  (|CallParentFunction))

(event Collision|EventActorBeginOverlap
  (params (OtherActor :type Actor%20Object%20Reference))
  (|CallParentFunction OtherActor) ; This node is disabled and will not be called.\nDrag off pins to build functionality.
)

(event EventTick
  (params (DeltaSeconds :type Float%20%28single-precision%29))
  (|CallParentFunction DeltaSeconds) ; This node is disabled and will not be called.\nDrag off pins to build functionality.
)

(event EventOnPickup
  (params (Object :type Object%20Object%20Reference))
  (bind _returnvalue (Transformation|GetActorLocation))
  (bind (_x _y _z) (Math|Vector|BreakVector _returnvalue))
  (bind _asphysics_ball_bp (Utilities|Casting|CastToPhysicsBallBP Object))
  (Physics|AddRadialImpulse (Variables|/Game/Blueprints/PhysicsBallBP.PhysicsBallBP_C|GetBall _asphysics_ball_bp) (Math|Vector|MakeVector _x _y (+ _z -5e+01)) 5e+02 5e+03 "RIF_Constant" true)
  (|CallParentFunction Object))

(fn ConstructionScript
  (|CallParentFunction))