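; Base pickup actor that awards its Points to the PhysicsBallBP when the ball overlaps its box.
; On pickup it plays a sound and particle effect and increases the ball's score.
; With UseNumberWidget on, it hides the mesh and animates a PickUpText widget showing the points; otherwise it destroys itself immediately.
; Any overlap, not just the ball's, also destroys the actor after a half-second delay.
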(event OnComponentBeginOverlap(Box)
  (params (OverlappedComponent :type Primitive%20Component%20Object%20Reference) (OtherActor :type Actor%20Object%20Reference) (OtherComp :type Primitive%20Component%20Object%20Reference) (OtherBodyIndex :type Integer) (bFromSweep :type Boolean) (SweepResult :type Hit%20Result%20Structure%20%28by%20ref%29))
  (CallFunction|OnPickup OtherActor)
  (Utilities|FlowControl|Delay 0.5)
  (Actor|DestroyActor))

(event EventBeginPlay
  (bind _pickuptext (Variables|Default|GetPickupText))
  (Rendering|SetVisibility _pickuptext false false)
  (bind _aspick_up_text (Utilities|Casting|CastToPickUpText (UserInterface|GetUserWidgetObject _pickuptext)))
  (Variables|/Game/Blueprints/Pickup/PickUpText.PickUpText_C|SetScore _aspick_up_text (Variables|Default|GetPoints)))

(event Collision|EventActorBeginOverlap
  (params (OtherActor :type Actor%20Object%20Reference)))

(event EventTick
  (params (DeltaSeconds :type Float%20%28single-precision%29)))

(fn ConstructionScript)

(fn OnPickup
  (params (Object :type Object%20Object%20Reference))
  (bind _asphysics_ball_bp (Utilities|Casting|CastToPhysicsBallBP Object))
  (Default|IncScore _asphysics_ball_bp (Variables|Default|GetPoints))
  (Audio|PlaySound2D (Variables|Default|GetPickupSound) 1.0 1.0 0.0 0 0)
  (Effects|SpawnEmitteratLocation (Variables|Default|GetPickup%20particle) (Transformation|GetActorLocation))
  (if (Variables|Default|GetuseNumberWidget)
    (Rendering|SetVisibility (Variables|Default|GetPickupText) true false)
    (Rendering|SetVisibility (Variables|Default|GetStaticMesh) false false)
    (bind _aspick_up_text (Utilities|Casting|CastToPickUpText (UserInterface|GetUserWidgetObject (Variables|Default|GetPickupText))))
    (UserInterface|Animation|PlayAnimation _aspick_up_text (Variables|/Game/Blueprints/Pickup/PickUpText.PickUpText_C|GetPickupAnimations _aspick_up_text) 0.0 1 "Forward" 1.0 false)
    (else
      (Actor|DestroyActor))))